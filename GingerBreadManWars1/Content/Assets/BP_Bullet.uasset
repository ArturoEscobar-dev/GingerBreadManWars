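; BP_Bullet is a projectile actor that destroys any enemy actor its Sphere begins overlapping.
; Shoot launches it by adding a force to the Sphere along the given direction, scaled by Force; it stores Damage but ignores SpeedMulti.
; The overlap kill does not use Damage.
; Active and Disabled toggle an IsActive flag and call Activate on the root component, without hiding or moving the bullet.
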(event `self.Sphere.OnComponentBeginOverlap`
  (params (OverlappedComponent :type "PrimitiveComponent Object Reference") (OtherActor :type "Actor Object Reference") (OtherComp :type "PrimitiveComponent Object Reference") (OtherBodyIndex :type Integer) (bFromSweep :type Boolean) (SweepResult :type "HitResult Structure (by ref)"))
  (bind _asenemy (cast `/Game/Blueprints/enemy` OtherActor))
  (`self.K2_DestroyActor` _asenemy))

(fn `Active`
  (`ActorComponent.Activate` (`self.DefaultSceneRoot`) true)
  (set `self.isActive` true))

(fn `Disabled`
  (`ActorComponent.Activate` (`self.DefaultSceneRoot`) false)
  (set `self.isActive` false))

(fn `Shoot`
  (params (Direction :type "Vector Structure") (`Speed Multi` :type "Float (double-precision)") (Damage :type "Float (double-precision)"))
  ;[1 1 1] Esta función dispara la bala
  (set `self.Damage` Damage)
  (`PrimitiveComponent.AddForce` (`self.Sphere`) (* Direction (`self.Force`)) "None" false))

(fn `UserConstructionScript`)